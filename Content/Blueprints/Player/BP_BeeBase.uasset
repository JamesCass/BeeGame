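; BP_BeeBase is the player bee, handling movement, ranged shooting and mouse cursor display.
; Enhanced Input drives world-axis movement, records Directionality and a held-move flag, and spawns BP_RangedWeapon at the Scene component's transform.
; Tick offsets the Weapon using roll and pitch from the deprojected mouse ray's look-at rotation, then calls RotateCharacter.
; RotateCharacter is empty, as its logic mapping RotationPoint yaw to four-way Directionality is disconnected.
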(event Input|EnhancedActionEvents|EnhancedInputActionIA_Move
  (params (ActionValue :type Vector%202D%20Structure) (ElapsedSeconds :type Float%20%28double-precision%29) (TriggeredSeconds :type Float%20%28double-precision%29) (InputAction :type Input%20Action%20Object%20Reference :default "/Game/Blueprints/Player/Input/IA_Move.IA_Move"))
  ;[0 0 0] Handles movement
  (:Triggered
    (Pawn|Input|AddMovementInput "1.000000,0.000000,0.000000" (.x ActionValue) false)
    (Pawn|Input|AddMovementInput "0.000000,-1.000000,0.000000" (.y ActionValue) false)
    (Variables|Default|SetDirectionality (Math|Vector2D|MakeVector2D (.x ActionValue) (.y ActionValue))))
  (:Started
    (Variables|Default|SetIsHoldingMove? true))
  (:Completed
    (Variables|Default|SetIsHoldingMove? false)))

(event Input|EnhancedActionEvents|EnhancedInputActionIA_Shoot
  (params (ActionValue :type Boolean) (ElapsedSeconds :type Float%20%28double-precision%29) (TriggeredSeconds :type Float%20%28double-precision%29) (InputAction :type Input%20Action%20Object%20Reference :default "/Game/Blueprints/Player/Input/IA_Shoot.IA_Shoot"))
  ;[0 0 0] Handles ranged attacking
  (:Triggered
    (Game|SpawnActorfromClass "/Game/Blueprints/BP_RangedWeapon.BP_RangedWeapon_C" (Transformation|GetWorldTransform (Variables|Default|GetScene)) "AlwaysSpawn" "MultiplyWithRoot" 0 0)))

(event EventTick
  (params (DeltaSeconds :type Float%20%28single-precision%29))
  (bind _returnvalue (Game|GetPlayerController 0))
  (bind (_worldlocation _worlddirection) (Game|Player|ConvertMouseLocationToWorldSpace _returnvalue))
  (bind _returnvalue_2 (* _worlddirection 1.0))
  (bind _returnvalue_3 (+ _worldlocation _returnvalue_2))
  (bind _returnvalue_4 (Math|Rotator|FindLookatRotation _worldlocation _returnvalue_3))
  (Variables|/Script/Engine.PlayerController|SetbShowMouseCursor _returnvalue true)
  (Transformation|SetRelativeLocation (Variables|Default|GetWeapon) (Math|Vector|MakeVector (.roll _returnvalue_4) (.pitch _returnvalue_4) 0.0) false false)
  (CallFunction|RotateCharacter))

(fn ConstructionScript)

(fn RotateCharacter)