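; BP_BeeParent is a player bee base with movement and ranged attack, using Enhanced Input.
; Move input drives world-axis movement and tracks a held flag, while attack spawns BP_RangedWeapon at the Scene component's transform.
; Each tick shows the cursor and writes the deprojected mouse ray's yaw into the Weapon's relative location Z.
; RotateCharacter then derives four-way Directionality from RotationPoint yaw, though some negative-yaw range checks can never pass.
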(event Input|EnhancedActionEvents|EnhancedInputActionIA_Move
  (params (ActionValue :type Vector%202D%20Structure) (ElapsedSeconds :type Float%20%28double-precision%29) (TriggeredSeconds :type Float%20%28double-precision%29) (InputAction :type Input%20Action%20Object%20Reference :default "/Game/Blueprints/Player/Input/IA_Move.IA_Move"))
  ;[0 0 0] Handles movement
  (:Triggered
    (Pawn|Input|AddMovementInput "1.000000,0.000000,0.000000" (.x ActionValue) false)
    (Pawn|Input|AddMovementInput "0.000000,-1.000000,0.000000" (.y ActionValue) false))
  (:Started
    (Variables|Default|SetIsHoldingMove? true))
  (:Canceled
    (Variables|Default|SetIsHoldingMove? false)))

(event Input|EnhancedActionEvents|EnhancedInputActionIA_Attack
  (params (ActionValue :type Boolean) (ElapsedSeconds :type Float%20%28double-precision%29) (TriggeredSeconds :type Float%20%28double-precision%29) (InputAction :type Input%20Action%20Object%20Reference :default "/Game/Blueprints/Player/Input/IA_Attack.IA_Attack"))
  ;[0 0 0] Handles ranged attacking
  (:Started
    (Game|SpawnActorfromClass "/Game/Blueprints/BP_RangedWeapon.BP_RangedWeapon_C" (Transformation|GetWorldTransform (Variables|Default|GetScene)) "AlwaysSpawn" "MultiplyWithRoot" 0 0)))

(event EventTick
  (params (DeltaSeconds :type Float%20%28single-precision%29))
  (bind _returnvalue (Game|GetPlayerController 0))
  (bind (_worldlocation _worlddirection) (Game|Player|ConvertMouseLocationToWorldSpace _returnvalue))
  (Variables|/Script/Engine.PlayerController|SetbShowMouseCursor _returnvalue true)
  (Transformation|SetRelativeLocation (Variables|Default|GetWeapon) (Math|Vector|MakeVector 0.0 0.0 (.yaw (Math|Rotator|FindLookatRotation _worldlocation (+ _worldlocation (* _worlddirection 1e+03))))) false false)
  (CallFunction|RotateCharacter))

(fn ConstructionScript)

(fn RotateCharacter
  (bind _rotationpoint (Variables|Default|GetRotationPoint))
  (bind _relativerotation (Variables|/Script/Engine.SceneComponent|GetRelativeRotation _rotationpoint))
  (if (and (> (.yaw _relativerotation) -45.0) (< (.yaw _relativerotation) 45.0))
    (Variables|Default|SetDirectionality "(X=1.000000,Y=0.000000)")
    (elif (and (> (.yaw _relativerotation) -45.0) (< (.yaw _relativerotation) -135.0))
      (Variables|Default|SetDirectionality "(X=0.000000,Y=1.000000)")
      (elif (and (> (.yaw _relativerotation) 45.0) (< (.yaw _relativerotation) 135.0))
        (Variables|Default|SetDirectionality "(X=0.000000,Y=-1.000000)")
        (elif (or (and (> (.yaw _relativerotation) 135.0) (< (.yaw _relativerotation) 1.8e+02)) (and (> (.yaw _relativerotation) -135.0) (< (.yaw _relativerotation) -1.8e+02)))
          (Variables|Default|SetDirectionality "(X=-1.000000,Y=0.000000)"))))))